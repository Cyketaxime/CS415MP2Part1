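; BP_PlayerController is a player controller that owns the on-screen HUD for health and score.
; On BeginPlay it creates the WBP_Health and WBP_Score widgets, stores references to them and adds both to the viewport.
; Its UpdateHealthBar and UpdateScore events forward current and max health or the score to the matching widget's setter.
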(event `self.ReceiveBeginPlay`
  (bind _returnvalue (`|CreateWidget` "/Game/LearningKit_Games/Blueprints/UI/WBP_Health.WBP_Health_C"))
  (bind _output_get (set `self.HealthBar` _returnvalue))
  (`UserWidget.AddToViewport` _output_get 0)
  (bind _returnvalue_2 (`|CreateWidget` "/Game/LearningKit_Games/Blueprints/UI/WBP_Score.WBP_Score_C"))
  (bind _output_get_2 (set `self.ScoreInfo` _returnvalue_2))
  (`UserWidget.AddToViewport` _output_get_2 0))

(event `UpdateHealthBar`
  (params (CurrHealth :type Integer) (MaxHealth :type Integer))
  (`/Game/LearningKit_Games/Blueprints/UI/WBP_Health.SetHealthBarInfo` (`self.HealthBar`) CurrHealth MaxHealth))

(event `UpdateScore`
  (params (Score :type Integer))
  (`/Game/LearningKit_Games/Blueprints/UI/WBP_Score.SetScoreInfo` (`self.ScoreInfo`) Score))

(fn `UserConstructionScript`)