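; Pursuer AI that either roams around its spawn point or chases the player and damages them on arrival.
; BeginPlay stores the spawn location and starts the behavior set by AIState.
; Perception updates switch between chase and roam based on distance to the player character.
; Each behavior is a self-restarting AIMoveTo loop with a short delay, and a successful chase also plays a particle effect and sound.
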(event `Chase Player`
  (`|AIMoveTo` self (0.0 0.0 0.0) (`GameplayStatics.GetPlayerCharacter` 0)
    (:`OnSuccess`
      (`GameplayStatics.ApplyDamage` (`GameplayStatics.GetPlayerCharacter` 0) 5.0)
      (`GameplayStatics.SpawnEmitterAtLocation` null (`self.K2_GetActorLocation` self))
      (`GameplayStatics.PlaySoundAtLocation` null (`self.K2_GetActorLocation` self) (struct) 1.0 1.0 0.0 null null null null)
      (`KismetSystemLibrary.Delay` 0.5)
      (`self.Chase Player`))))

(event `Roam`
  (`|AIMoveTo` self (`NavigationSystemV1.K2_GetRandomReachablePointInRadius` (`self.SpawnLocation`) 500.0 null null) null
    (:`OnSuccess`
      (`KismetSystemLibrary.Delay` 0.5)
      (`self.Roam`))))

(event `self.ReceiveBeginPlay`
  (set `self.SpawnLocation` (`self.K2_GetActorLocation`))
  (switch `/Game/LearningKit_Games/Blueprints/BaseClasses/EAIState` (`self.AIState`)
    (:`NewEnumerator1`
      (`self.Roam`))
    (:`NewEnumerator2`
      (`self.Chase Player`))))

(event `self.AIPerception.OnPerceptionUpdated`
  (params (UpdatedActors :type "Array of Actor Object Reference (by ref)"))
  (for _array_element UpdatedActors
    (bind _asbp_learning_kit_player_character (cast `/Game/LearningKit_Games/Blueprints/PlayerCharacter/BP_LearningKit_PlayerCharacter` _array_element))
    (if (<= (`KismetMathLibrary.Vector_Distance` (`self.K2_GetActorLocation` _asbp_learning_kit_player_character) (`self.K2_GetActorLocation` self)) 500.0)
      (set `self.AIState` "NewEnumerator2")
      (`self.Chase Player`)
      (else
        (set `self.AIState` "NewEnumerator1")
        (`self.Roam`)))))

(fn `UserConstructionScript`)